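; BP_Laser is an interactable laser hazard that damages and pushes back actors that overlap it.
; On overlap, it runs the parent logic, then its ability system component applies the BP_GE_LaserDamage gameplay effect to the overlapping actor's ability system component.
; It then sends that actor a Movement.Pushback gameplay event carrying the push force as event magnitude, leaving the movement response to whatever handles the event.
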(event `self.ReceiveActorBeginOverlap`
  (params (OtherActor :type "Actor Object Reference"))
  (bind _output_get (set `self.TargetActor` OtherActor))
  (`parent.ReceiveActorBeginOverlap` OtherActor)
  (`AbilitySystemComponent.BP_ApplyGameplayEffectToTarget` :`self` (`self.AbilitySystemComponent`) :`GameplayEffectClass` "/Game/GAS/GameplayEffects/BP_GE_LaserDamage.BP_GE_LaserDamage_C" :`Target` (`AbilitySystemBlueprintLibrary.GetAbilitySystemComponent` _output_get))
  (set `self.PushForce` 600.0)
  (`AbilitySystemBlueprintLibrary.SendGameplayEventToActor` (`self.TargetActor`) (struct :`TagName` "Movement.Pushback") (make `GameplayEventData` (struct) null null null null (struct) (struct) (struct) (`self.PushForce`))))

(fn `UserConstructionScript`
  (`parent.UserConstructionScript`))